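; BP_DeskProcessing is a desk actor that can be claimed by a worker and tinted to that worker's team color.
; BeginPlay creates a dynamic material on the mesh, and ColorizeDeskToWorker sets its color parameter from the assigned worker.
; Box overlap queries resolve nearby points: the first player spawn point found and a random worker dropoff point.
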(event EventBeginPlay
  (bind _returnvalue (Rendering|Material|CreateDynamicMaterialInstance (Variables|Default|GetStaticMesh) 0 (Rendering|Material|GetMaterial (Variables|Default|GetStaticMesh) 0) "None" :!class /Script/Engine.PrimitiveComponent))
  (Variables|Default|SetDesk%20Paint _returnvalue))

(event Collision|EventActorBeginOverlap
  (params (OtherActor :type Actor%20Object%20Reference)))

(event EventTick
  (params (DeltaSeconds :type Float%20%28single-precision%29)))

(fn ConstructionScript)

(fn AssignWorkertoDesk
  (params (Worker :type Master%20Character%20Object%20Reference) (Is%20Claimed :type Boolean))
  (Variables|Default|SetWorker Worker)
  (Variables|Default|SetIs%20Claimed Is%20Claimed))

(fn GetSpawnPoint
  (bind _box (Variables|Default|GetBox))
  (bind _overlappingactors (Collision|GetOverlappingActors _box "/Game/Blueprints/BP_PlayerSpawnPoint.BP_PlayerSpawnPoint_C" :!class /Script/Engine.PrimitiveComponent))
  (if (== (Utilities|Array|Length _overlappingactors) 0)
    (return 0)
    (else
      (bind _asbp_player_spawn_point (Utilities|Casting|CastToBP_PlayerSpawnPoint (Utilities|Array|Get(acopy) _overlappingactors)))
      (return _asbp_player_spawn_point))))

(fn ColorizeDesktoWorker
  (bind _worker (Variables|Default|GetWorker))
  (Utilities|IsValid _worker
    (:Is%20Valid
      (Rendering|Material|SetVectorParameterValue (Variables|Default|GetDesk%20Paint) "Desk Color" (Variables|/Game/Blueprints/MasterCharacter.MasterCharacter_C|GetTeamColor _worker) :!class /Script/Engine.MaterialInstanceDynamic))))

(fn GetDropoffPoint
  (bind _box (Variables|Default|GetBox))
  (bind _overlappingactors (Collision|GetOverlappingActors _box "/Game/Blueprints/BP_WorkerDropoffPoint.BP_WorkerDropoffPoint_C" :!class /Script/Engine.PrimitiveComponent))
  (if (== (Utilities|Array|Length _overlappingactors) 0)
    (return 0)
    (else
      (bind _asbp_worker_dropoff_point (Utilities|Casting|CastToBP_WorkerDropoffPoint (.OutItem (Utilities|Array|Random _overlappingactors))))
      (return _asbp_worker_dropoff_point))))