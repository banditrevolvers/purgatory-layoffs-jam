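; Master character for office workers that fight, collect work reports and turn them in at their own desk for rating.
; StatsComponent handles health, mana, regeneration and sprint cost, while carried reports reduce walk speed.
; Attacks take montage, damage and hit sound from the child-actor weapon, with bare-hand fallbacks.
; Death scatters carried work and updates the AI blackboard; revive resets stats, equips fists and returns the worker to its desk spawn.
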(event Custom|Attack
  (bind _stops_movement (CallFunction|WeaponStopsMovement?))
  ;[1 1 1] Attack
  (bind _attacking (CallFunction|IsAttacking?))
  (if (not _attacking)
    (Variables|Combat|SetIs%20Attacking true)
    (if _stops_movement
      (Pawn|Components|CharacterMovement|DisableMovement (Variables|Character|GetCharacterMovement)))
    (bind _returnvalue (Animation|PlayAnimMontage (Weapon|GetWeaponMontage) 1.0 "None"))
    (Utilities|FlowControl|Delay _returnvalue)
    (if _stops_movement
      (Pawn|Components|CharacterMovement|SetMovementMode (Variables|Character|GetCharacterMovement) "MOVE_Walking" 0))
    (Variables|Combat|SetIs%20Attacking false)))

(event Custom|Kill%20Character
  (params (Death%20Causer :type Actor%20Object%20Reference) (Elimination :type Boolean))
  ;[1 1 1] Kill Character
  (if Elimination
    (Variables|Default|SetIs%20Eliminated true))
  (bind _alive (CallFunction|IsAlive?))
  (if _alive
    (Math|Integer|IncrementInt (Variables|/Game/Blueprints/StatsComponent.StatsComponent_C|GetDeath%20Count (Variables|Default|GetStatsComponent))
      (:%20%20
        (Collision|SetCollisionEnabled (Variables|Collision|GetCapsuleComponent) "NoCollision")
        (Variables|Default|SetIs%20Alive false)
        (CallFunction|UpdateBlackboardStatus)
        (CallFunction|DropItems)
        (Audio|PlaySoundatLocation (Variables|Default|GetDeath%20Sound) (Transformation|GetActorLocation) "0, 0, 0" 1.0 1.0 0.0 0 0 0 0)
        (CallFunction|StopAttacking)
        (Pawn|Components|CharacterMovement|DisableMovement (Variables|Character|GetCharacterMovement))
        (bind _returnvalue (Animation|PlayAnimMontage (Variables|Default|GetDeath%20Montage) 1.0 "None"))
        (Utilities|FlowControl|Delay (- _returnvalue 0.5))
        (Variables|Default|SetIs%20Waiting%20Respawn true)
        (Variables|/Script/Engine.SkeletalMeshComponent|SetbPauseAnims (Variables|Character|GetMesh) true)
        (Utilities|IsValid (Variables|Default|GetHealth%20Widget%20Ref)
          (:Is%20Valid
            (Widget|SetVisibility (Variables|Default|GetHealth%20Widget%20Ref) "Hidden"))
          (:Is%20Not%20Valid
            _))
        (Default|CallWorkerDied self Death%20Causer)
        (Decal|HideDecal)))))

(event Custom|Revive%20Character
  (bind _health_widget_ref (Variables|Default|GetHealth%20Widget%20Ref))
  ;[1 1 1] Revive Character
  (Default|ResetStats (Variables|Default|GetStatsComponent))
  (Utilities|IsValid (Variables|Default|GetHealth%20Widget%20Ref)
    (:Is%20Valid
      (Widget|SetVisibility _health_widget_ref "Visible")
      (Default|UpdateInformation _health_widget_ref))
    (:Is%20Not%20Valid
      (CallFunction|SetWidgetReference)))
  (Variables|Default|SetIs%20Alive true)
  (CallFunction|UpdateBlackboardStatus)
  (Variables|Default|SetIs%20Waiting%20Respawn false)
  (Decal|ShowDecal)
  (Pawn|Components|CharacterMovement|SetMovementMode (Variables|Character|GetCharacterMovement) "MOVE_Walking" 0)
  (Collision|SetCollisionEnabled (Variables|Collision|GetCapsuleComponent) "QueryAndPhysics")
  (CallFunction|EquipFistWeapon)
  (bind _found_desk (CallFunction|GetWorkDesk))
  (Variables|/Script/Engine.SkeletalMeshComponent|SetbPauseAnims (Variables|Character|GetMesh) false)
  (Utilities|IsValid _found_desk
    (:Is%20Valid
      (bind _player_spawn_point (Default|GetSpawnPoint _found_desk))
      (Utilities|IsValid _player_spawn_point
        (:Is%20Valid
          (Transformation|SetActorLocation (Transformation|GetActorLocation _player_spawn_point) false false))))))

(event EventBeginPlay
  (bind _health_widget_ref (Variables|Default|GetHealth%20Widget%20Ref))
  ;[1 1 1] Begin Play
  (bind _asbp_top_down_character (Utilities|Casting|CastToBP_TopDownCharacter (Game|GetPlayerCharacter 0)))
  (Variables|Default|SetPlayer%20Character%20Reference _asbp_top_down_character)
  (Variables|Default|SetMovement%20Base%20Speed (Variables|/Script/Engine.CharacterMovementComponent|GetMaxWalkSpeed (Variables|Character|GetCharacterMovement)))
  (Speed|AdjustMovementSpeed)
  (CallFunction|SetWidgetReference)
  (Variables|/Game/Blueprints/WBP_WorkerFloatingWidget.WBP_WorkerFloatingWidget_C|SetMaster%20Character%20Actor (Variables|Default|GetHealth%20Widget%20Ref) self)
  (Utilities|IsValid _health_widget_ref
    (:Is%20Valid
      (Default|UpdateInformation _health_widget_ref))))

(event EventItemPickedUp
  (params (Item%20Picked%20Up :type Actor%20Object%20Reference))
  (bind _health_widget_ref (Variables|Default|GetHealth%20Widget%20Ref))
  ;[1 1 1] Event Item Picked Up
  (bind _asbp_work_collectable (Utilities|Casting|CastToBP_WorkCollectable Item%20Picked%20Up))
  (Variables|Default|SetCarriedReports (+ (Variables|Default|GetCarriedReports) (Variables|/Game/Blueprints/BP_WorkCollectable.BP_WorkCollectable_C|GetWork%20Value _asbp_work_collectable)))
  (Default|DestroyWork _asbp_work_collectable)
  (Speed|AdjustMovementSpeed)
  (Utilities|IsValid _health_widget_ref
    (:Is%20Valid
      (Default|UpdateInformation _health_widget_ref))))

(event EventTick
  (params (DeltaSeconds :type Float%20%28single-precision%29))
  (Utilities|FlowControl|Sequence
    (:then_0
      ;[1 1 1] Sprinting Mana Usage
      (if (Variables|Default|GetIs%20Sprinting)
        (Utilities|FlowControl|Delay 1.0)
        ;;[1 1 1] Stop if no mana left to sprint
        (if (<= (Variables|/Game/Blueprints/StatsComponent.StatsComponent_C|GetCurrentMana (Variables|Default|GetStatsComponent)) 0.0)
          (Variables|Default|SetIs%20Sprinting false)
          (Speed|AdjustMovementSpeed)
          (else
            ;;[1 1 1] Use Mana while sprinting
            (Default|TickSprintUsage (Variables|Default|GetStatsComponent))))))
    (:then_1
      (Utilities|FlowControl|Delay 1.0)
      (bind _alive (CallFunction|IsAlive?))
      (if _alive
        (Utilities|FlowControl|Sequence
          (:then_0
            ;[1 1 1] Mana Regeneration
            (if (not (Variables|Default|GetIs%20Sprinting))
              (Default|TickManaRegeneration (Variables|Default|GetStatsComponent))))
          (:then_1
            ;[1 1 1] Health Regneneration
            (Default|TickHealthRegeneration (Variables|Default|GetStatsComponent))))))))

(event EventDidDamagetoWorker
  ;[1 1 1] Increase Rating on Damage To Worker
  (Variables|Default|SetRating (+ (Variables|/Game/Blueprints/StatsComponent.StatsComponent_C|GetRatingOnHit (Variables|Default|GetStatsComponent)) (Variables|Default|GetRating))))

(event Game|Damage|EventAnyDamage
  (params (Damage :type Float%20%28single-precision%29) (DamageType :type Damage%20Type%20Object%20Reference) (InstigatedBy :type Controller%20Object%20Reference) (DamageCauser :type Actor%20Object%20Reference))
  (bind _health_widget_ref (Variables|Default|GetHealth%20Widget%20Ref))
  ;[1 1 1] AnyDamage
  (if (Variables|Default|GetIs%20Alive)
    (Default|TakeDamage (Variables|Default|GetStatsComponent) Damage)
    (Utilities|IsValid DamageCauser
      (:Is%20Valid
        (Class|BPIWokerInterface|DidDamagetoWorker(Message) DamageCauser))
      (:Is%20Not%20Valid
        _))
    (Utilities|IsValid _health_widget_ref
      (:Is%20Valid
        (Default|UpdateInformation _health_widget_ref)
        (Utilities|FlowControl|DoOnce false :!label _label
          (:Completed
            (if (CallFunction|CheckifDead)
              (CallFunction|KillCharacter DamageCauser false)
              (goto _label Reset)
              (else
                (Pawn|Components|CharacterMovement|DisableMovement (Variables|Character|GetCharacterMovement))
                (bind _returnvalue (Animation|PlayAnimMontage (CallFunction|GetFlinchMontage) 1.0 "None"))
                (Utilities|FlowControl|Delay _returnvalue)
                (Pawn|Components|CharacterMovement|SetMovementMode (Variables|Character|GetCharacterMovement) "MOVE_Walking" 0)
                (goto _label Reset)))))))))

(event Collision|EventActorBeginOverlap
  (params (OtherActor :type Actor%20Object%20Reference))
  ;[0.09201 0.09201 0.09201] Actor Overlap
)

(fn ConstructionScript)

(fn GetMovementSpeed
  (return (* (Variables|Default|GetMovement%20Base%20Speed) (/ (- 1e+02 (Speed|GetReportSpeedPercentageMod)) 1e+02))))

(fn GrabbingItem
  (params (Grab%20Actor :type Actor%20Object%20Reference))
  (bind _asbp_work_collectable (Utilities|Casting|CastToBP_WorkCollectable Grab%20Actor))
  (Variables|Default|SetCarriedReports (+ (Variables|Default|GetCarriedReports) (Variables|/Game/Blueprints/BP_WorkCollectable.BP_WorkCollectable_C|GetWork%20Value _asbp_work_collectable)))
  (Default|DestroyWork _asbp_work_collectable)
  (Speed|AdjustMovementSpeed))

(fn GetCurrentRating
  (return (Math|Float|Round (+ (* (Variables|Default|GetTurnedInWork) 10) (Variables|Default|GetRating)))))

(fn AssignWorkDetails
  (params (Worker%20Struct :type S%20Worker%20Structure))
  (bind _statscomponent (Variables|Default|GetStatsComponent))
  (Utilities|FlowControl|Sequence
    (:then_0
      ;[1 1 1] Set Name
      (Variables|Default|SetCharacter%20Name (.name Worker%20Struct)))
    (:then_1
      ;[1 1 1] Set Health and Mana
      (Default|SetCurrentandMaxHealth _statscomponent (.health Worker%20Struct))
      (Default|SetCurrentandMaxMana _statscomponent (.mana Worker%20Struct)))
    (:then_2
      ;[1 1 1] Set Mesh
      (Class|SkinnedMeshComponent|SetSkeletalMesh (Variables|Character|GetMesh) (.meshmodel Worker%20Struct) true))
    (:then_3
      ;[1 1 1] Assign Materials to Mesh
      (for (_array_element _array_index) (.material Worker%20Struct)
        (Rendering|Material|SetMaterial (Variables|Character|GetMesh) _array_index _array_element)))
    (:then_4
      (return))))

(fn GetWeaponMontage
  (bind _asbp_weapon_collectable (Utilities|Casting|CastToBP_WeaponCollectable (Variables|/Script/Engine.ChildActorComponent|GetChildActor (Variables|Default|GetChildActor)))
    (:then
      (return (Variables|/Game/Blueprints/BP_WeaponCollectable.BP_WeaponCollectable_C|GetWeapon%20Attack%20Montage _asbp_weapon_collectable)))
    (:CastFailed
      (return "/Game/Characters/Attack_PrimaryA__1__Montage.Attack_PrimaryA__1__Montage"))))

(fn GetWeaponHitSound
  (bind _asbp_weapon_collectable (Utilities|Casting|CastToBP_WeaponCollectable (Variables|/Script/Engine.ChildActorComponent|GetChildActor (Variables|Default|GetChildActor)))
    (:then
      (return (Variables|/Game/Blueprints/BP_WeaponCollectable.BP_WeaponCollectable_C|GetWeapon%20Hit%20Sound _asbp_weapon_collectable)))
    (:CastFailed
      (return "/Game/Sound/Punch.Punch"))))

(fn GetFlinchMontage
  (return "/Game/Characters/Impact_mixamo_com_Montage.Impact_mixamo_com_Montage"))

(fn GetWeaponDamage
  (bind _asbp_weapon_collectable (Utilities|Casting|CastToBP_WeaponCollectable (Variables|/Script/Engine.ChildActorComponent|GetChildActor (Variables|Default|GetChildActor)))
    (:then
      (return (Default|GenerateDamage _asbp_weapon_collectable)))
    (:CastFailed
      (return (Math|Random|RandomFloatinRange 5.0 6.0)))))

(fn GetWorkDesk
  (bind _outactors (Actor|GetAllActorsOfClass "/Game/Blueprints/BP_DeskProcessing.BP_DeskProcessing_C"))
  (bind _array_element (Utilities|Array|ForEachLoopwithBreak _outactors :!label _label)
    (:LoopBody
      (if (== (Variables|/Game/Blueprints/BP_DeskProcessing.BP_DeskProcessing_C|GetWorker _array_element) self)
        (LocalVariables|SetFound%20Worker%20Desk _array_element)
        (goto _label Break)))
    (:Completed
      (return (LocalVariables|GetFound%20Worker%20Desk)))))

(fn GetLevel
  (return (Variables|Default|GetLevel)))

(fn SetWidgetReference
  (bind _aswbp_worker_floating_widget (Utilities|Casting|CastToWBP_WorkerFloatingWidget (UserInterface|GetUserWidgetObject (Variables|Default|GetWidget)))
    (:then
      (Variables|Default|SetHealth%20Widget%20Ref _aswbp_worker_floating_widget))
    (:CastFailed
      _))
  (return))

(fn CheckifDead
  (return (<= (Variables|/Game/Blueprints/StatsComponent.StatsComponent_C|GetCurrentHealth (Variables|Default|GetStatsComponent)) 0.0)))

(fn GetReportSpeedPercentageMod
  (return (Math|Float|Clamp(Float) (* (Variables|Default|GetCarriedReports) (Variables|Default|GetSpeed%20Reduction%20Per%20Report)) 0.0 95.0)))

(fn AdjustMovementSpeed
  (bind _movement (Speed|GetMovementSpeed))
  (if (Variables|Default|GetIs%20Sprinting)
    (if (< _movement (Variables|Default|GetMovement%20Base%20Speed))
      (Variables|/Script/Engine.CharacterMovementComponent|SetMaxWalkSpeed (Variables|Character|GetCharacterMovement) (Variables|Default|GetMovement%20Base%20Speed))
      (else
        (Variables|/Script/Engine.CharacterMovementComponent|SetMaxWalkSpeed (Variables|Character|GetCharacterMovement) (* _movement 1.5))))
    (else
      (Variables|/Script/Engine.CharacterMovementComponent|SetMaxWalkSpeed (Variables|Character|GetCharacterMovement) (Speed|GetMovementSpeed)))))

(fn WeaponStopsMovement?
  (return false))

(fn EquipFistWeapon
  (bind _childactor (Variables|Default|GetChildActor))
  (bind _childactor_2 (Variables|/Script/Engine.ChildActorComponent|GetChildActor _childactor))
  (ChildActorComponent|SetChildActorClass _childactor "/Game/Blueprints/BP_FistWeapon.BP_FistWeapon_C")
  (Utilities|IsValid _childactor_2
    (:Is%20Valid
      (Actor|SetOwner _childactor_2 self))))

(fn UpdateBlackboardStatus
  (bind _returnvalue (AI|GetBlackboard 0))
  (Utilities|IsValid _returnvalue
    (:Is%20Valid
      (bind _alive (CallFunction|IsAlive?))
      (AI|Components|Blackboard|SetValueasBool _returnvalue (Utilities|Name|MakeLiteralName "IsAlive") _alive)
      ;[1 1 1] If Not alive, then set no enemy and clear focus
      (if (not _alive)
        (AI|Components|Blackboard|ClearValue _returnvalue (Utilities|Name|MakeLiteralName "EnemyActor"))
        (bind _asaicontroller (Utilities|Casting|CastToAIController (Pawn|GetController)))
        (AI|ClearFocus _asaicontroller)))))

(fn UpdateDecalTeamColor
  (Rendering|Material|SetVectorParameterValue (Variables|Default|GetDecal%20Paint) "Team Color" (Variables|Default|GetTeamColor) :!class /Script/Engine.MaterialInstanceDynamic))

(fn ShowDecal
  (Rendering|SetVisibility (Variables|Default|GetDecal) true false))

(fn HideDecal
  (Rendering|SetVisibility (Variables|Default|GetDecal) false false))

(fn StopAttacking
  (Variables|Combat|SetIs%20Attacking false)
  (Animation|StopAnimMontage 0))

(fn CreateDecal
  (bind _returnvalue (Rendering|Material|CreateDynamicMaterialInstance (Variables|Default|GetDecal) :!class /Script/Engine.DecalComponent))
  (Variables|Default|SetDecal%20Paint _returnvalue))

(fn DropItems
  (CallFunction|DropWork))

(fn DropWork
  (bind _returnvalue (Transformation|GetActorLocation))
  (bind _health_widget_ref (Variables|Default|GetHealth%20Widget%20Ref))
  (bind _randomlocation (AI|Navigation|GetRandomReachablePointinRadius _returnvalue 2.5e+02 0 0))
  (if (> (Variables|Default|GetCarriedReports) 0)
    (LocalVariables|SetWork%20to%20drop (Variables|Default|GetCarriedReports))
    (while (> (LocalVariables|GetWork%20to%20drop) 0)
      (Math|Integer|DecrementInt (LocalVariables|GetWork%20to%20drop)
        (:%20%20
          (Audio|PlaySoundatLocation "/Game/Sound/Paper_Crumple_Crumpling_Scrunch_Crunch_Sfx_Cue.Paper_Crumple_Crumpling_Scrunch_Crunch_Sfx_Cue" _randomlocation "0, 0, 0" 0.6 1.0 0.0 "/Game/Sound/NewSoundAttenuation.NewSoundAttenuation" 0 0 0)
          (Game|SpawnActorfromClass "/Game/Blueprints/BP_WorkCollectable.BP_WorkCollectable_C" (Math|Transform|MakeTransform _randomlocation "0, 0, 0" "1.000000,1.000000,1.000000") "AdjustIfPossibleButAlwaysSpawn" 0 (Math|Random|RandomFloatinRange 15.0 3e+01) 0))))
    (Variables|Default|SetCarriedReports 0)
    (Speed|AdjustMovementSpeed)
    (Utilities|IsValid _health_widget_ref
      (:Is%20Valid
        (Default|UpdateInformation _health_widget_ref)))))

(fn DepositWork
  (params (Desk%20Object :type Actor%20Object%20Reference))
  (bind _found_desk (CallFunction|GetWorkDesk))
  (Utilities|IsValid _found_desk
    (:Is%20Valid
      (if (and (== _found_desk Desk%20Object) (> (Variables|Default|GetCarriedReports) 0))
        (bind _output_get (Variables|Default|SetTurnedInWork (+ (Variables|Default|GetTurnedInWork) (Variables|Default|GetCarriedReports))))
        (Variables|Default|SetCarriedReports 0)
        (Development|PrintString (Utilities|String|Append (Utilities|String|ToString(Text) (Variables|Default|GetCharacter%20Name)) "Turned in work " (Utilities|String|ToString(Integer) _output_get)) false false)
        (return true)
        (else
          _)))
    (:Is%20Not%20Valid
      _))
  (return false))

(fn IsAlive?
  (return (Variables|Default|GetIs%20Alive)))

(fn IsAttacking?
  (return (Variables|Combat|GetIs%20Attacking)))