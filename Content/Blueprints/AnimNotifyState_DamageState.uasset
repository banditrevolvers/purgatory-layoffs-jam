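; An anim notify state that marks the damage window of an attack animation on a MasterCharacter.
; On begin it calls WeaponActive on the BP_WeaponCollectable held in the character's ChildActor component, and on end it calls WeaponDeactive.
; Both handlers cast the mesh owner and the child actor, doing nothing when either cast fails.
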(fn ReceivedNotifyBegin
  (params (MeshComp :type Skeletal%20Mesh%20Component%20Object%20Reference) (Animation :type Anim%20Sequence%20Base%20Object%20Reference) (TotalDuration :type Float%20%28single-precision%29) (EventReference :type Anim%20Notify%20Event%20Reference%20Structure%20%28by%20ref%29))
  (bind _asmaster_character (Utilities|Casting|CastToMasterCharacter (Components|GetOwner MeshComp)))
  (bind _asbp_weapon_collectable (Utilities|Casting|CastToBP_WeaponCollectable (Variables|/Script/Engine.ChildActorComponent|GetChildActor (Variables|/Game/Blueprints/MasterCharacter.MasterCharacter_C|GetChildActor _asmaster_character))))
  (Default|WeaponActive _asbp_weapon_collectable)
  (return true))

(fn ReceivedNotifyEnd
  (params (MeshComp :type Skeletal%20Mesh%20Component%20Object%20Reference) (Animation :type Anim%20Sequence%20Base%20Object%20Reference) (EventReference :type Anim%20Notify%20Event%20Reference%20Structure%20%28by%20ref%29))
  (bind _asmaster_character (Utilities|Casting|CastToMasterCharacter (Components|GetOwner MeshComp)))
  (bind _asbp_weapon_collectable (Utilities|Casting|CastToBP_WeaponCollectable (Variables|/Script/Engine.ChildActorComponent|GetChildActor (Variables|/Game/Blueprints/MasterCharacter.MasterCharacter_C|GetChildActor _asmaster_character))))
  (Default|WeaponDeactive _asbp_weapon_collectable)
  (return true))