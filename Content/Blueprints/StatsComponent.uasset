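; StatsComponent holds a character's health, mana and respawn timer, with functions to set, damage, regenerate and reset them.
; Tick-style functions apply sprint mana drain, health and mana regeneration and respawn countdown in clamped steps, relying on outside callers because its event graph is empty.
; The respawn delay grows with DeathCount, and CanRespawn reports when it reaches zero.
; Damage clamps health to a fixed ceiling rather than MaxHealth.
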(event EventBeginPlay)

(event EventTick
  (params (DeltaSeconds :type Float%20%28single-precision%29)))

(fn SetCurrentandMaxHealth
  (params (Health :type Float%20%28double-precision%29))
  (Variables|Default|SetCurrentHealth Health)
  (Variables|Default|SetMaxHealth Health))

(fn SetCurrentandMaxMana
  (params (CurrentMana :type Float%20%28double-precision%29))
  (Variables|Default|SetCurrentMana CurrentMana)
  (Variables|Default|SetMaxMana CurrentMana))

(fn TakeDamage
  (params (Damage :type Float%20%28double-precision%29))
  (Variables|Default|SetCurrentHealth (Math|Float|Clamp(Float) (- (Variables|Default|GetCurrentHealth) Damage) 0.0 1e+03)))

(fn GetHealthPercent
  (return (/ (Variables|Default|GetCurrentHealth) (Variables|Default|GetMaxHealth))))

(fn ResetStats
  (CallFunction|SetCurrentandMaxHealth (Variables|Default|GetMaxHealth))
  (CallFunction|SetCurrentandMaxMana (Variables|Default|GetMaxMana)))

(fn TickSprintUsage
  (Variables|Default|SetCurrentMana (Math|Float|Clamp(Float) (- (Variables|Default|GetCurrentMana) (Variables|Default|GetSprintManaUsage)) 0.0 (Variables|Default|GetMaxMana))))

(fn TickManaRegeneration
  (if (not (== (Variables|Default|GetCurrentMana) (Variables|Default|GetMaxMana)))
    (Variables|Default|SetCurrentMana (Math|Float|Clamp(Float) (+ (Variables|Default|GetCurrentMana) (Variables|Default|GetManaRegeneration)) 0.0 (Variables|Default|GetMaxMana)))))

(fn TickHealthRegeneration
  (if (not (== (Variables|Default|GetCurrentHealth) (Variables|Default|GetMaxHealth)))
    (Variables|Default|SetCurrentHealth (Math|Float|Clamp(Float) (+ (Variables|Default|GetCurrentHealth) (Variables|Default|GetHealthRegeneration)) 0.0 (Variables|Default|GetMaxHealth)))))

(fn RestartRespawnTimer
  (Variables|Default|SetRespawn%20Timer (+ (Variables|Default|GetStarting%20Respawn%20Timer) (* (Variables|Default|GetDeath%20Count) 5))))

(fn TickRespawnTimer
  (Variables|Default|SetRespawn%20Timer (Math|Float|Clamp(Float) (- (Variables|Default|GetRespawn%20Timer) 1.0) 0.0 2.5e+02)))

(fn CanRespawn
  (return (== (Variables|Default|GetRespawn%20Timer) 0.0)))