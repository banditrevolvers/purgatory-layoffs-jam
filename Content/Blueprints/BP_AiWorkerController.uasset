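; AI controller for worker characters that runs BT_AiWorker and feeds it Blackboard keys.
; A looping one-second needs check sets a work flag and sends report carriers toward their desk's dropoff point.
; When perception senses a character, a randomized score from health, personality tags and carried reports decides whether it becomes EnemyActor.
; Losing perception starts a timer that clears the target and focus.
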(event OnTargetPerceptionUpdated(AIPerception)
  (params (Actor :type Actor%20Object%20Reference) (Stimulus :type AI%20Stimulus%20Structure))
  (bind _output_get (Variables|Default|SetSensed%20Actor Actor))
  ;[1 1 1] See Player
  (bind _asmaster_character (Utilities|Casting|CastToMasterCharacter _output_get))
  (if (.bSuccessfullySensed (Utilities|Struct|BreakAIStimulus Stimulus))
    (bind (_wants_to_fight _total_fighting_chance) (CallFunction|ConsiderFightingWorker _asmaster_character))
    (Development|PrintString (Utilities|String|ToString(Text) (Utilities|Text|FormatText "{persona} saw {personb} and {chance} and {scrappy}" (Variables|/Game/Blueprints/MasterCharacter.MasterCharacter_C|GetCharacter%20Name (Variables|Default|GetMy%20Master%20Character)) (Variables|/Game/Blueprints/MasterCharacter.MasterCharacter_C|GetCharacter%20Name _asmaster_character) _total_fighting_chance _wants_to_fight)) false false "(R=0.353746,G=0.192942,B=1.000000,A=1.000000)")
    (if _wants_to_fight
      (bind _output_get_2 (Variables|Default|SetCurrent%20Target _asmaster_character))
      (AI|Components|Blackboard|SetValueasObject (Variables|Default|GetBlackboard) (Utilities|Name|MakeLiteralName "EnemyActor") _output_get_2))
    (else
      (bind _returnvalue (Utilities|Time|SetTimerbyEvent (delegate Custom|Lose%20Target) (Variables|Default|GetLost%20Sight%20Time%20Amount)))
      (Variables|Default|SetLose%20%20Sight%20Timer _returnvalue))))

(event Custom|Lose%20Target
  ;[1 1 1] On Loss of Target
  (Variables|Default|SetCurrent%20Target 0)
  (AI|Components|Blackboard|ClearValue (Variables|Default|GetBlackboard) (Utilities|Name|MakeLiteralName "EnemyActor"))
  (AI|ClearFocus))

(event EventBeginPlay
  (bind _returnvalue (Utilities|Time|SetTimerbyFunctionName 0 "Assess Needs" 1.0 true))
  (Variables|Default|SetAssess%20Needs%20Timer _returnvalue))

(event EventTick
  (params (DeltaSeconds :type Float%20%28single-precision%29)))

(event EventPossess
  (params (PossessedPawn :type Pawn%20Object%20Reference))
  ;[1 1 1] On Possess
  (AI|RunBehaviorTree "/Game/AI/BT_AiWorker.BT_AiWorker")
  (Variables|Default|SetMy%20Blackboard (AI|GetBlackboard 0))
  (bind _output_get (Variables|Default|SetMy%20Possessed%20Pawn PossessedPawn))
  (bind _asmaster_character (Utilities|Casting|CastToMasterCharacter _output_get))
  (Variables|Default|SetMy%20Master%20Character _asmaster_character))

(fn ConstructionScript)

(fn AssessNeeds
  (bind _asworker_character (Utilities|Casting|CastToWorkerCharacter (Pawn|GetControlledPawn)))
  (LocalVariables|SetWorker%20Ref _asworker_character)
  (Utilities|FlowControl|Sequence
    (:then_0
      ;[1 1 1] Target Needs to find work
      (if (< (Variables|/Game/Blueprints/MasterCharacter.MasterCharacter_C|GetCarriedReports (LocalVariables|GetWorker%20Ref)) 8)
        (Variables|Default|SetNeeds%20Work true)
        (else
          (Variables|Default|SetNeeds%20Work false))))
    (:then_1
      ;[1 1 1] Check if need to drop off work
      (if (>= (Variables|/Game/Blueprints/MasterCharacter.MasterCharacter_C|GetCarriedReports (LocalVariables|GetWorker%20Ref)) 1)
        ;[1 1 1] Check if their work desk exists
        (bind _found_desk (Default|GetWorkDesk (LocalVariables|GetWorker%20Ref)))
        (Utilities|IsValid _found_desk
          (:Is%20Valid
            (Utilities|FlowControl|Sequence
              (:then_0
                (AI|Components|Blackboard|SetValueasBool (Variables|Default|GetMy%20Blackboard) (Utilities|Name|MakeLiteralName "NeedsGoHome") true))
              (:then_1
                (AI|Components|Blackboard|SetValueasVector (Variables|Default|GetBlackboard) (Utilities|Name|MakeLiteralName "TargetLocation") (Transformation|GetActorLocation (Default|GetDropoffPoint _found_desk)))))))
        (else
          (AI|Components|Blackboard|SetValueasBool (Variables|Default|GetMy%20Blackboard) (Utilities|Name|MakeLiteralName "NeedsGoHome") false))))))

(fn ConsiderFightingWorker
  (params (Other%20Worker :type Master%20Character%20Object%20Reference))
  (Utilities|FlowControl|Sequence
    (:then_0
      ;[1 1 1] If I have more health
      (if (> (Variables|/Game/Blueprints/StatsComponent.StatsComponent_C|GetCurrentHealth (Variables|/Game/Blueprints/MasterCharacter.MasterCharacter_C|GetStatsComponent (Variables|Default|GetMy%20Master%20Character))) (Variables|/Game/Blueprints/StatsComponent.StatsComponent_C|GetCurrentHealth (Variables|/Game/Blueprints/MasterCharacter.MasterCharacter_C|GetStatsComponent Other%20Worker)))
        (LocalVariables|SetFighting%20Chance (+ (LocalVariables|GetFighting%20Chance) 0.25))))
    (:then_1
      ;[1 1 1] If I am aggressive
      (if (Actor|ActorHasTag (Variables|Default|GetMy%20Master%20Character) "Personality.Aggressive")
        (LocalVariables|SetFighting%20Chance (+ (LocalVariables|GetFighting%20Chance) 0.5))))
    (:then_2
      ;[1 1 1] If I am Pacifist
      (if (Actor|ActorHasTag (Variables|Default|GetMy%20Master%20Character) "Personality.Pacifist")
        (LocalVariables|SetFighting%20Chance (- (LocalVariables|GetFighting%20Chance) 0.25))))
    (:then_3
      ;[1 1 1] IF they have more reports than me
      (if (> (Variables|/Game/Blueprints/MasterCharacter.MasterCharacter_C|GetCarriedReports Other%20Worker) (Variables|/Game/Blueprints/MasterCharacter.MasterCharacter_C|GetCarriedReports (Variables|Default|GetMy%20Master%20Character)))
        (LocalVariables|SetFighting%20Chance (+ (LocalVariables|GetFighting%20Chance) 0.25))))
    (:then_4
      ;[1 1 1] If other is at low health
      (if (< (Variables|/Game/Blueprints/StatsComponent.StatsComponent_C|GetCurrentHealth (Variables|/Game/Blueprints/MasterCharacter.MasterCharacter_C|GetStatsComponent Other%20Worker)) 15.0)
        (LocalVariables|SetFighting%20Chance (- (LocalVariables|GetFighting%20Chance) 0.15))))
    (:then_5
      (return (< (Math|Random|RandomFloat) (Math|Float|Clamp(Float) (+ (LocalVariables|GetFighting%20Chance) (Math|Random|RandomFloatinRange 0.0 0.25)))) (+ (LocalVariables|GetFighting%20Chance) (Math|Random|RandomFloatinRange 0.0 0.25))))))