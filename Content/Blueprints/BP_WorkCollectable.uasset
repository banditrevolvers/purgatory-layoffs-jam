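; BP_WorkCollectable is a collectable "work" actor that is linked to the spawner that created it.
; On BeginPlay it sets its life span from DespawnTimer when that value is positive, so it can expire automatically.
; DestroyWork clears the SpawnedWork reference on a valid WorkSpawner and then destroys the actor.
; Timed expiry does not route through DestroyWork, and the overlap and tick events are unused.
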(event EventBeginPlay
  (if (> (Variables|Default|GetDespawn%20Timer) 0.0)
    (Actor|SetLifeSpan (Variables|Default|GetDespawn%20Timer))))

(event Collision|EventActorBeginOverlap
  (params (OtherActor :type Actor%20Object%20Reference)))

(event EventTick
  (params (DeltaSeconds :type Float%20%28single-precision%29)))

(fn ConstructionScript)

(fn DestroyWork
  (Utilities|IsValid (Variables|Default|GetWork%20Spawner)
    (:Is%20Valid
      (Variables|/Game/Blueprints/BP_WorkSpawnZone.BP_WorkSpawnZone_C|SetSpawned%20Work (Variables|Default|GetWork%20Spawner) 0))
    (:Is%20Not%20Valid
      _))
  (Actor|DestroyActor))