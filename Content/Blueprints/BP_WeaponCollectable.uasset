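; Weapon actor that deals random damage within a min-max range to overlapped actors tagged "Damageable", excluding its owner.
; WeaponActive and WeaponDeactive events switch the Collider between overlap-all and no collision, opening and closing the hit window.
; Each hit plays a sound at the target and applies damage credited to the owner, with a DoOnce and short Delay throttling repeat hits.
; Character casts on overlap only drive debug prints comparing owner and target.
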(event OnComponentBeginOverlap(Collider)
  (params (OverlappedComponent :type Primitive%20Component%20Object%20Reference) (OtherActor :type Actor%20Object%20Reference) (OtherComp :type Primitive%20Component%20Object%20Reference) (OtherBodyIndex :type Integer) (bFromSweep :type Boolean) (SweepResult :type Hit%20Result%20Structure%20%28by%20ref%29))
  (bind _returnvalue (Components|GetOwner))
  (bind _asbp_top_down_character (Utilities|Casting|CastToBP_TopDownCharacter _returnvalue)
    (:then
      (bind _asmaster_character (Utilities|Casting|CastToMasterCharacter OtherActor)
        (:then
          (Development|PrintString (Utilities|String|Append (Utilities|String|ToString(Text) (Variables|/Game/Blueprints/MasterCharacter.MasterCharacter_C|GetCharacter%20Name _asbp_top_down_character)) "vs" (Utilities|String|ToString(Text) (Variables|/Game/Blueprints/MasterCharacter.MasterCharacter_C|GetCharacter%20Name _asmaster_character))) true true "(R=0.522090,G=1.000000,B=0.284141,A=1.000000)")
          (if (!= _asmaster_character _asbp_top_down_character)
            (Development|PrintString "Different Person!" true true "(R=0.522090,G=1.000000,B=0.284141,A=1.000000)")))
        (:CastFailed
          _)))
    (:CastFailed
      _))
  (if (!= OtherActor _returnvalue)
    (if (Actor|ActorHasTag OtherActor "Damageable")
      (Utilities|FlowControl|DoOnce false :!label _label
        (:Completed
          (Audio|PlaySoundatLocation (Variables|Default|GetWeapon%20Hit%20Sound) (Transformation|GetActorLocation OtherActor) "0, 0, 0" 1.0 1.0 0.0 0 0 0 0)
          (Game|Damage|ApplyDamage OtherActor (CallFunction|GenerateDamage) 0 _returnvalue)
          (Utilities|FlowControl|Delay 0.5)
          (goto _label Reset))))))

(event Custom|Weapon%20Active
  (Collision|SetCollisionProfileName (Variables|Default|GetCollider) "OverlapAll" true :!class /Script/Engine.PrimitiveComponent))

(event Custom|Weapon%20Deactive
  (Collision|SetCollisionEnabled (Variables|Default|GetCollider) "NoCollision"))

(event EventBeginPlay
  (|CallParentFunction) ; This node is disabled and will not be called.\nDrag off pins to build functionality.
)

(event Collision|EventActorBeginOverlap
  (params (OtherActor :type Actor%20Object%20Reference))
  (|CallParentFunction OtherActor) ; This node is disabled and will not be called.\nDrag off pins to build functionality.
)

(event EventTick
  (params (DeltaSeconds :type Float%20%28single-precision%29))
  (|CallParentFunction DeltaSeconds) ; This node is disabled and will not be called.\nDrag off pins to build functionality.
)

(fn ConstructionScript
  (|CallParentFunction))

(fn GenerateDamage
  (return (Math|Random|RandomFloatinRange (Variables|Default|GetDamageMin) (Variables|Default|GetDamageMax))))