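; BP_WorkSpawnZone is a spawn point that keeps one BP_WorkCollectable available in the level.
; It spawns the first collectable silently on BeginPlay at its Arrow's location and gives it a back-reference to the spawner.
; While that collectable is invalid, Tick decrements a countdown once per frame, so the delay is framerate-dependent.
; At zero it respawns the collectable with a sound and resets the countdown.
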(event EventBeginPlay
  (CallFunction|SpawnWork false)
  (Variables|Default|SetCurrent%20Countdown (Variables|Default|GetSpawn%20Countdown)))

(event Collision|EventActorBeginOverlap
  (params (OtherActor :type Actor%20Object%20Reference)))

(event EventTick
  (params (DeltaSeconds :type Float%20%28single-precision%29))
  (Utilities|IsValid (Variables|Default|GetSpawned%20Work)
    (:Is%20Not%20Valid
      (bind _result (Math|Integer|DecrementInt (Variables|Default|GetCurrent%20Countdown))
        (:%20%20
          (if (<= _result 0)
            (CallFunction|SpawnWork true)
            (Variables|Default|SetCurrent%20Countdown (Variables|Default|GetSpawn%20Countdown))))))))

(fn ConstructionScript)

(fn SpawnWork
  (params (Noisy%20Spawn :type Boolean))
  (bind _arrow (Variables|Default|GetArrow))
  (bind _returnvalue (Transformation|GetWorldLocation _arrow))
  (Utilities|IsValid (Variables|Default|GetSpawned%20Work)
    (:Is%20Not%20Valid
      (if Noisy%20Spawn
        (Audio|PlaySoundatLocation "/Game/Sound/WorkRespawn.WorkRespawn" _returnvalue "0, 0, 0" 1.0 1.0 0.0 0 0 0 0))
      (bind _returnvalue_2 (Game|SpawnActorfromClass "/Game/Blueprints/BP_WorkCollectable.BP_WorkCollectable_C" (Math|Transform|MakeTransform _returnvalue (Transformation|GetActorRotation) "1.000000,1.000000,1.000000") "Undefined" 0 0.0 0))
      (bind _output_get (Variables|Default|SetSpawned%20Work _returnvalue_2))
      (Variables|/Game/Blueprints/BP_WorkCollectable.BP_WorkCollectable_C|SetWork%20Spawner _output_get self))))